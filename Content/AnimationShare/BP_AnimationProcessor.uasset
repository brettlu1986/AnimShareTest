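; Animation Sharing state processor that tells the sharing system which animation state each BP_ModularCharacter2 actor is in.
; ProcessActorState casts the actor, returns its GetCurrentState as an integer, and flags processing only when that differs from the state passed in.
; GetAnimationStateEnum supplies Enum_State as the state enum.
; The on-demand input is unused, and disconnected draft logic for on-demand states remains in the graph.
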(fn ProcessActorState
  (params (InActor :type Actor%20Object%20Reference) (CurrentState :type Byte :default 0) (OnDemandState :type Byte :default 0))
  (LocalVariables|SetbProcess false)
  (bind _asbp_modular_character_2 (Utilities|Casting|CastToBP_ModularCharacter2 InActor))
  (if (!= CurrentState (Default|GetCurrentState _asbp_modular_character_2))
    (LocalVariables|SetbProcess true))
  (return (Math|Conversions|ToInteger(Byte) (Default|GetCurrentState _asbp_modular_character_2)) (LocalVariables|GetbProcess)))

(fn GetAnimationStateEnum
  (return "/Game/Blueprint/Enum_State.Enum_State"))