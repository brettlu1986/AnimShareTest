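; Spawner actor that places grids of modular characters from its own location, in a standard or an AnimShare variant with separate classes.
; Spawn functions fill the row/column grid at once or spawn a single AnimShare test character.
; CalPoses builds shuffled grid positions for staggered spawning through nested delay loops.
; Those staggered chains are disconnected, so both AsyncSpawn events do nothing.
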(event Custom|AsyncSpawnCharacters)

(event Custom|AsyncSpawnAnimShareCharacters)

(event EventBeginPlay)

(event Collision|EventActorBeginOverlap
  (params (OtherActor :type Actor%20Object%20Reference)))

(event EventTick
  (params (DeltaSeconds :type Float%20%28single-precision%29)))

(fn ConstructionScript)

(fn SpawnCharacters
  (bind _returnvalue (Transformation|GetActorLocation))
  (for _index (range 0 (- (Variables|Default|GetColumnCount) 1))
    (for _index_2 (range 0 (- (Variables|Default|GetRowCount) 1))
      (CallFunction|SpawnCharacter (Math|Vector|MakeVector (+ (* _index (Variables|Default|GetCharacterSpaceInColumn)) (.x _returnvalue)) (+ (* _index_2 (Variables|Default|GetCharacterSpaceInRow)) (.y _returnvalue)) (.z _returnvalue)) (Transformation|GetActorRotation)))))

(fn SpawnCharacter
  (params (Loc :type Vector) (Rot :type Rotator))
  (Game|SpawnActorfromClass "/Game/Blueprint/BP_ModularCharracter1.BP_ModularCharracter1_C" (Math|Transform|MakeTransform Loc Rot) "Undefined" 0 0))

(fn CalPoses
  (bind _returnvalue (Transformation|GetActorLocation))
  (for _index (range 0 (- (Variables|Default|GetColumnCount) 1))
    (for _index_2 (range 0 (- (Variables|Default|GetRowCount) 1))
      (Utilities|Array|Add (Variables|Default|GetRandPos) (Math|Vector|MakeVector (+ (* _index (Variables|Default|GetCharacterSpaceInColumn)) (.x _returnvalue)) (+ (* _index_2 (Variables|Default|GetCharacterSpaceInRow)) (.y _returnvalue)) (.z _returnvalue)))))
  (Utilities|Array|Shuffle (Variables|Default|GetRandPos)))

(fn SpawnAnimShareCharacters
  (bind _returnvalue (Transformation|GetActorLocation))
  (for _index (range 0 (- (Variables|Default|GetColumnCount) 1))
    (for _index_2 (range 0 (- (Variables|Default|GetRowCount) 1))
      (CallFunction|SpawnAnimShareCharacter (Math|Vector|MakeVector (+ (* _index (Variables|Default|GetCharacterSpaceInColumn)) (.x _returnvalue)) (+ (* _index_2 (Variables|Default|GetCharacterSpaceInRow)) (.y _returnvalue)) (.z _returnvalue)) (Transformation|GetActorRotation)))))

(fn SpawnAnimShareCharacter
  (params (Loc :type Vector) (Rot :type Rotator))
  (Game|SpawnActorfromClass "/Game/Blueprint/BP_ModularCharacter2.BP_ModularCharacter2_C" (Math|Transform|MakeTransform Loc Rot) "Undefined" 0 0))

(fn SpawnAnimTestShareCharacer
  (CallFunction|SpawnAnimShareCharacter "-80.000000, 0,90.000000" "0,90.000000, 0"))