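; BP_AnimGameMode is a game mode Blueprint that controls which PlayerStart a player spawns at.
; Its ChoosePlayerStart function fills the PlayerStarts array from the level's PlayerStart actors whenever that array is empty, then reuses it.
; It returns the first start tagged "PlayStart", or nothing if none matches.
; The event graph and construction script contain no logic.
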(event EventBeginPlay)

(event EventTick
  (params (DeltaSeconds :type Float%20%28single-precision%29)))

(fn ConstructionScript)

(fn ChoosePlayerStart
  (params (Player :type Controller%20Object%20Reference))
  (if (== (Utilities|Array|Length (Variables|Default|GetPlayerStarts)) 0)
    (bind _outactors (Actor|GetAllActorsOfClass "/Script/Engine.PlayerStart"))
    (Variables|Default|SetPlayerStarts _outactors))
  (for _array_element (Variables|Default|GetPlayerStarts)
    (if (Utilities|Name|Equal(Name) (Variables|/Script/Engine.PlayerStart|GetPlayerStartTag _array_element) "PlayStart")
      (return _array_element)))
  (return 0))