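; BP_ModularCharacter2 is a modular character whose Head, Hands and Downbody parts follow the main Mesh through Master Pose, set in the construction script.
; From BeginPlay, the AnimSwitchTimer timeline's forward event track steps a State enum, wrapping to the first value, and GetCurrentState exposes it.
; UpdateHeadShowState is called on each change but does nothing, as its widget text update is disconnected, as is a significance debug print.
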(event EventBeginPlay
  (|CallParentFunction)
  (Variables|Default|SetState "NewEnumerator0")
  (CallFunction|UpdateHeadShowState)
  (bind _direction (Timeline|AnimSwitchTimer Play)
    (:EventStateTimeLine
      (if (Utilities|Enum|Equal(Enum) _direction "Forward")
        (if (> (+ (Variables|Default|GetState) 1) (Utilities|Enum|LiteralenumEnum_State "NewEnumerator4"))
          (Variables|Default|SetState "NewEnumerator0")
          (else
            (Variables|Default|SetState (Utilities|Enum|ByteToEnumEnum_State (+ (Variables|Default|GetState) 1)))))
        (CallFunction|UpdateHeadShowState)))))

(event Collision|EventActorBeginOverlap
  (params (OtherActor :type Actor%20Object%20Reference)))

(event EventTick
  (params (DeltaSeconds :type Float%20%28single-precision%29))
  (|CallParentFunction 0.0))

(fn ConstructionScript
  (Class|SkinnedMeshComponent|SetMasterPoseComponent (Variables|Default|Gethead) (Variables|Character|GetMesh) false))

(fn GetCurrentState
  (return (Variables|Default|GetState)))

(fn UpdateHeadShowState)